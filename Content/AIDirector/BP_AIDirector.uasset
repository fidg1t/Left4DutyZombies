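; AI Director actor that rates how stressed the player is and maps that to a director state.
; Every Tick it blends player health, ammo, recent damage, kill rate and alive-enemy ratio into a weighted, clamped Stress score.
; Thresholds turn Stress into one of four states, with the previous state printed for debugging.
; A separate event spawns a random pooled enemy at a random spawn point, but nothing here calls it.
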(event Custom|SpawnEnemyAtRandomPoint
  (Game|SpawnActorfromClass (.OutItem (Utilities|Array|Random (Variables|Default|GetEnemyPool))) (Transformation|GetActorTransform (.OutItem (Utilities|Array|Random (Variables|Default|GetSpawnPoints)))) "Undefined" "MultiplyWithRoot" 0 0))

(event EventBeginPlay
  (bind _returnvalue (Actor|GetActorOfClass "/Game/FirstPerson/Blueprints/BP_FirstPersonCharacter.BP_FirstPersonCharacter_C"))
  (Variables|Default|SetPlayerRef _returnvalue))

(event Collision|EventActorBeginOverlap
  (params (OtherActor :type Actor%20Object%20Reference)))

(event EventTick
  (params (DeltaSeconds :type Float%20%28single-precision%29))
  (CallFunction|CalculateStress)
  (Development|PrintString (Utilities|String|EnumtoString (Variables|Default|GetDirectorState)))
  (if (< (Variables|GameState|GetStress) (Variables|GameState|GetCalmThreshold))
    (Variables|Default|SetDirectorState "NewEnumerator0")
    (elif (< (Variables|GameState|GetStress) (Variables|GameState|GetBuildThreshold))
      (Variables|Default|SetDirectorState "NewEnumerator1")
      (elif (< (Variables|GameState|GetStress) (Variables|GameState|GetPeakThreshold))
        (Variables|Default|SetDirectorState "NewEnumerator2")
        (elif true
          (Variables|Default|SetDirectorState "NewEnumerator3"))))))

(fn ConstructionScript)

(fn CalculateHealthFactor
  (bind _playerref (Variables|Default|GetPlayerRef))
  (return (- 1.0 (/ (Variables|/Game/FirstPerson/Blueprints/BP_FirstPersonCharacter.BP_FirstPersonCharacter_C|GetHealth _playerref) (Variables|/Game/FirstPerson/Blueprints/BP_FirstPersonCharacter.BP_FirstPersonCharacter_C|GetMaxHealth _playerref)))))

(fn CalculateAmmoFactor
  (bind _playerref (Variables|Default|GetPlayerRef))
  (return (- 1.0 (/ (Math|Conversions|ToFloat(Integer) (Variables|/Game/FirstPerson/Blueprints/BP_FirstPersonCharacter.BP_FirstPersonCharacter_C|GetAmmo _playerref)) (Math|Conversions|ToFloat(Integer) (Variables|/Game/FirstPerson/Blueprints/BP_FirstPersonCharacter.BP_FirstPersonCharacter_C|GetMaxAmmo _playerref))))))

(fn CalculateEnemyFactor
  (return (/ (Math|Conversions|ToFloat(Integer) (Variables|Default|GetAliveEnemies)) (Math|Conversions|ToFloat(Integer) (Variables|Default|GetMaxAliveEnemies)))))

(fn CalculateRecentDamageFactor
  (return (/ (Variables|/Game/FirstPerson/Blueprints/BP_FirstPersonCharacter.BP_FirstPersonCharacter_C|GetRecentDamage (Variables|Default|GetPlayerRef)) 1e+02)))

(fn CalculatePerformanceFactor
  (return (- 1.0 (/ (Variables|/Game/FirstPerson/Blueprints/BP_FirstPersonCharacter.BP_FirstPersonCharacter_C|GetKillsPerMinute (Variables|Default|GetPlayerRef)) 5e+01))))

(fn CalculateStress
  (bind _healthfactor (CallFunction|CalculateHealthFactor))
  (Variables|Factors|SetHealthFactor _healthfactor)
  (bind _ammofactor (CallFunction|CalculateAmmoFactor))
  (Variables|Factors|SetAmmoFactor _ammofactor)
  (bind _enemyfactor (CallFunction|CalculateEnemyFactor))
  (Variables|Factors|SetEnemyFactor _enemyfactor)
  (bind _recentdamagefactor (CallFunction|CalculateRecentDamageFactor))
  (Variables|Factors|SetRecentDamageFactor _recentdamagefactor)
  (bind _performancefactor (CallFunction|CalculatePerformanceFactor))
  (Variables|Factors|SetPerformanceFactor _performancefactor)
  (bind _output_get (Variables|GameState|SetStress (Math|Float|Clamp(Float) (+ (* (Variables|Factors|GetHealthFactor) 3e+01) (* (Variables|Factors|GetAmmoFactor) 2e+01) (* (Variables|Factors|GetEnemyFactor) 25.0) (* (Variables|Factors|GetRecentDamageFactor) 15.0) (* (Variables|Factors|GetPerformanceFactor) 1e+01)) 0.0 1e+02)))
  (return _output_get))